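; BP_WheelChar is a player-controlled physics wheel that is steered, braked and boosted through forces and impulses.
; BeginPlay picks the mesh from the game instance's WheelIdx, but first overwrites it with 8, so W010 always loads.
; A/D or the left_F/right_F events push sideways above the wheel's origin.
; Space cancels spin and S adds velocity-dependent forward acceleration, each gated by and resetting a game-instance timer.
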(event Custom|right_F
  (bind _wheel (Variables|Default|Getwheel))
  (bind _returnvalue (Transformation|GetWorldLocation _wheel))
  (bind (_x _y _z) (Math|Vector|BreakVector _returnvalue))
  (Class|PrimitiveComponent|AddForceatLocation _wheel "0.000000,2000000.000000,0.000000" (Math|Vector|MakeVector _x _y (+ _z 7e+01)) "None"))

(event Custom|left_F
  (bind _wheel (Variables|Default|Getwheel))
  (bind _returnvalue (Transformation|GetWorldLocation _wheel))
  (bind (_x _y _z) (Math|Vector|BreakVector _returnvalue))
  (Class|PrimitiveComponent|AddForceatLocation _wheel "0,-2000000.000000,0.000000" (Math|Vector|MakeVector _x _y (+ _z 7e+01)) "None"))

(event EventBeginPlay
  (bind _wheel (Variables|Default|Getwheel))
  (bind _askusa_game_instance (Utilities|Casting|CastTokusaGameInstance (Game|GetGameInstance)))
  (Variables|/Script/wheelSpin.kusaGameInstance|SetWheelIdx _askusa_game_instance 8)
  (switch int (Variables|/Script/wheelSpin.kusaGameInstance|GetWheelIdx _askusa_game_instance)
    (:Default
      (Components|StaticMesh|SetStaticMesh _wheel "/Game/utils/meshes/wheel/w001.w001" :!label _label))
    (:0
      (goto _label))
    (:1
      (Components|StaticMesh|SetStaticMesh _wheel "/Game/utils/meshes/wheel/w002.w002"))
    (:2
      (Components|StaticMesh|SetStaticMesh _wheel "/Game/utils/meshes/wheel/w003.w003"))
    (:3
      (Components|StaticMesh|SetStaticMesh _wheel "/Game/utils/meshes/wheel/w004.w004"))
    (:4
      (Components|StaticMesh|SetStaticMesh _wheel "/Game/utils/meshes/wheel/w006.w006"))
    (:5
      (Components|StaticMesh|SetStaticMesh _wheel "/Game/utils/meshes/wheel/w007.w007"))
    (:6
      (Components|StaticMesh|SetStaticMesh _wheel "/Game/utils/meshes/wheel/w008.w008"))
    (:7
      (Components|StaticMesh|SetStaticMesh _wheel "/Game/utils/meshes/wheel/w009.w009"))
    (:8
      (Components|StaticMesh|SetStaticMesh _wheel "/Game/utils/meshes/wheel/w010.w010"))))

(event Collision|EventActorBeginOverlap
  (params (OtherActor :type Actor%20Object%20Reference)))

(event EventTick
  (params (DeltaSeconds :type Float%20%28single-precision%29)))

(event Input|KeyboardEvents|D
  (params (Key :type Key%20Structure))
  (bind _wheel (Variables|Default|Getwheel))
  (bind _returnvalue (Transformation|GetWorldLocation _wheel))
  (bind (_x _y _z) (Math|Vector|BreakVector _returnvalue))
  (:Pressed
    (Class|PrimitiveComponent|AddForceatLocation _wheel "0.000000,2000000.000000,0.000000" (Math|Vector|MakeVector _x _y (+ _z 7e+01)) "None")))

(event Input|KeyboardEvents|A
  (params (Key :type Key%20Structure))
  (bind _wheel (Variables|Default|Getwheel))
  (bind _returnvalue (Transformation|GetWorldLocation _wheel))
  (bind (_x _y _z) (Math|Vector|BreakVector _returnvalue))
  (:Pressed
    (Class|PrimitiveComponent|AddForceatLocation _wheel "0,-2000000.000000,0.000000" (Math|Vector|MakeVector _x _y (+ _z 7e+01)) "None")))

(event Input|KeyboardEvents|S
  (params (Key :type Key%20Structure))
  (bind _wheel (Variables|Default|Getwheel))
  (bind _returnvalue (Transformation|GetComponentVelocity _wheel))
  (bind (_x _y _z) (Math|Vector|BreakVector _returnvalue))
  (:Pressed
    (bind _askusa_game_instance (Utilities|Casting|CastTokusaGameInstance (Game|GetGameInstance)))
    (if (>= (Variables|/Script/wheelSpin.kusaGameInstance|GetSpeedTimer _askusa_game_instance) 5e+02)
      (Variables|/Script/wheelSpin.kusaGameInstance|SetSpeedTimer _askusa_game_instance 0.0)
      (if (> _x 5e+02)
        (Physics|AddForce _wheel (Math|Vector|MakeVector (* _x 3e+01) _y _z) "None" true)
        (else
          (Physics|AddForce _wheel "100000.000000, 0, 0" "None" true))))))

(event Input|KeyboardEvents|SpaceBar
  (params (Key :type Key%20Structure))
  (bind _wheel (Variables|Default|Getwheel))
  (:Pressed
    (bind _askusa_game_instance (Utilities|Casting|CastTokusaGameInstance (Game|GetGameInstance)))
    (if (>= (Variables|/Script/wheelSpin.kusaGameInstance|GetBrakeTimer _askusa_game_instance) 5e+02)
      (Variables|/Script/wheelSpin.kusaGameInstance|SetBrakeTimer _askusa_game_instance 0.0)
      (Class|PrimitiveComponent|AddAngularImpulseinDegrees _wheel (* (Physics|GetPhysicsAngularVelocityinDegrees _wheel "None") -1.0) "None" true))))

(fn ConstructionScript)